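; Base dice actor that rolls with physics and works out which value it landed on.
; RollDice randomizes rotation, enables physics on DiceMesh, and starts a looping timer that polls the transform until it stops changing.
; An upward line trace from the mesh, able to hit itself, then converts the hit component's name to an integer, stores it in DiceData's CurrentRoll and prints it.
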(event `RollDice`
  (bind _returnvalue (`self.K2_SetActorRotation` (`KismetMathLibrary.RandomRotator` true) true))
  (`PrimitiveComponent.SetSimulatePhysics` (`self.DiceMesh`) _returnvalue)
  (set `self.PreviousTransform` (`self.GetTransform`))
  (bind _returnvalue_2 (`KismetSystemLibrary.K2_SetTimerDelegate` (`|CreateDelegate` :!event `Check is Rolling`) 0.1 true false 0.1))
  (set `self.RollCheckTimer` _returnvalue_2))

(event `Check is Rolling`
  (if (== (`self.GetTransform`) (`self.PreviousTransform`))
    (`KismetSystemLibrary.K2_ClearAndInvalidateTimerHandle` (`self.RollCheckTimer`))
    (`self.Get Roll Result`)
    (else
      (set `self.PreviousTransform` (`self.GetTransform`)))))

(event `Get Roll Result`
  (bind _returnvalue (`SceneComponent.K2_GetComponentLocation` (`self.DiceMesh`)))
  (bind _outhit (`KismetSystemLibrary.LineTraceSingle` :`Start` _returnvalue :`End` (`KismetMathLibrary.MakeVector` (.x _returnvalue) (.y _returnvalue) (+ (.z _returnvalue) 200.0)) :`TraceChannel` "TraceTypeQuery1" :`bTraceComplex` true :`DrawDebugType` "Persistent" :`bIgnoreSelf` false))
  (bind _structout (setmembers `/Game/Blueprints/Dice/S_DiceData` :`StructRef` (`self.DiceData`) :`CurrentRoll` (`KismetStringLibrary.Conv_StringToInt` (`KismetSystemLibrary.GetObjectName` (`.HitComponent` (`GameplayStatics.BreakHitResult` _outhit))))))
  (`KismetSystemLibrary.PrintString` (`KismetStringLibrary.Concat_StrStr` "Rolled: " (`KismetStringLibrary.Conv_IntToString` (`.CurrentRoll_7_99659F794855A09B9250029CED0EA4DE` (break `/Game/Blueprints/Dice/S_DiceData` _structout)))) true true (struct :`G` 0.66 :`B` 1.0 :`A` 1.0) 15.0))

(fn `UserConstructionScript`)