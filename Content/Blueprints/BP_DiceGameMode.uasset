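; BP_DiceGameMode is a game mode for a dice game that sets up and rolls the starting dice on BeginPlay.
; It sets a string-based phase to StartTurn and calls StartTurn, which currently only prints a debug message.
; It then spawns a BP_Dice for each StartingDice entry in a spaced row, assigns its side count through DiceData, stores it in SpawnedDice and rolls it.
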(event `self.ReceiveBeginPlay`
  (set `self.CurrentPhase` "StartTurn")
  (`self.StartTurn`)
  (for (_array_element _array_index) (`self.StartingDice`)
    (bind _returnvalue (`|SpawnActorFromClass` "/Game/Blueprints/Dice/BP_Dice.BP_Dice_C" (`KismetMathLibrary.MakeTransform` (`KismetMathLibrary.MakeVector` 500.0 (+ (* _array_index 150) 2000.0) 150.0)) "Undefined" "MultiplyWithRoot" null null))
    (setmembers `/Game/Blueprints/Dice/S_DiceData` :`StructRef` (`/Game/Blueprints/Dice/BP_Dice.DiceData` _returnvalue) :`Sides` _array_element)
    (`KismetArrayLibrary.Array_Add` (`self.SpawnedDice`) _returnvalue)
    (`/Game/Blueprints/Dice/BP_Dice.RollDice` _returnvalue)))

(fn `StartTurn`
  (`KismetSystemLibrary.PrintString` "Starting Turn"))

(fn `UserConstructionScript`)